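; BP_MissionAreaVolume is a volume that damages the player for staying outside the mission area too long.
; When a BP_Marine leaves the Trigger, it flags the marine as outside and starts a timer set by SecondsBeforePlayerDeath.
; An actor overlap by a marine clears the flag and cancels the timer.
; If the timer expires, Kill Player applies fixed damage to player character 0, regardless of which marine left.
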(event OnComponentEndOverlap(Trigger)
  (params (OverlappedComponent :type Primitive%20Component%20Object%20Reference) (OtherActor :type Actor%20Object%20Reference) (OtherComp :type Primitive%20Component%20Object%20Reference) (OtherBodyIndex :type Integer))
  ;[1 1 1] Player Leaves Mission Area
  (bind _asbp_marine (Utilities|Casting|CastToBP_Marine OtherActor))
  (Variables|/Game/Blueprint/Pawns/BP_Marine.BP_Marine_C|SetOutside%20Mission%20Area _asbp_marine true)
  (Utilities|Time|SetTimerbyFunctionName 0 "Kill Player" (Variables|Default|GetSeconds%20Before%20Player%20Death)))

(event EventBeginPlay)

(event Collision|EventActorBeginOverlap
  (params (OtherActor :type Actor%20Object%20Reference))
  ;[1 1 1] Player Enters Mission Area
  (bind _asbp_marine (Utilities|Casting|CastToBP_Marine OtherActor))
  (Variables|/Game/Blueprint/Pawns/BP_Marine.BP_Marine_C|SetOutside%20Mission%20Area _asbp_marine false)
  (Utilities|Time|ClearTimerbyFunctionName 0 "Kill Player"))

(event EventTick
  (params (DeltaSeconds :type Float%20%28single-precision%29)))

(fn ConstructionScript)

(fn KillPlayer
  (Game|Damage|ApplyDamage (Game|GetPlayerCharacter 0) 1e+02 0 0))